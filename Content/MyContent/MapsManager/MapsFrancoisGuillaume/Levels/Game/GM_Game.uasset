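; GM_Game is the game mode that admits players to a networked session and puts each one in a sports car.
; Each arrival joins a controller list and restarts a short retriggerable delay, then session settings are read.
; Once the player count reaches the connection limit, surplus players are kicked as "server full", the session is updated, and listed controllers possess newly spawned cars.
; Logout removes the controller from the list.
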(event `self.HandleStartingNewPlayer`
  (params (NewPlayer :type "PlayerController Object Reference"))
  (`KismetArrayLibrary.Array_AddUnique` (`self.playerControllers`) NewPlayer)
  (`KismetSystemLibrary.RetriggerableDelay` 2.0)
  (bind (_numconnections _numprivateconnections _bislan _bisdedicated _ballowinvites _ballowjoininprogress _bisanticheatenabled _builduniqueid _extrasettings) (`AdvancedSessionsLibrary.GetSessionSettings`)
    (:`OnSuccess`
      (if (> (`KismetArrayLibrary.Array_Length` (`GameStateBase.PlayerArray` (`GameplayStatics.GetGameState`))) _numconnections)
        (bind (_arrayindex _arrayelement) (`/Engine/EditorBlueprintResources/StandardMacros.ReverseForEachLoop` (`self.playerControllers`))
          (:`LoopBody`
            (if (>= _arrayindex _numconnections)
              (`AdvancedSessionsLibrary.KickPlayer` _arrayelement "Serveur Complet")))
          (:`Completed`
            (`UpdateSessionCallbackProxyAdvanced.UpdateSession` _extrasettings _numconnections :!label _label
              (:`OnSuccess`
                (for _array_element (`self.playerControllers`)
                  (bind _returnvalue (`|SpawnActorFromClass` "/Game/VehicleTemplate/Blueprints/SportsCar/SportsCar_Pawn.SportsCar_Pawn_C" (`KismetMathLibrary.MakeTransform` (0.0 0.0 0.0)) "Undefined" "OverrideRootScale" null null))
                  (`Controller.Possess` _array_element _returnvalue))))))
        (elif (== (`KismetArrayLibrary.Array_Length` (`GameStateBase.PlayerArray` (`GameplayStatics.GetGameState`))) _numconnections)
          (goto _label))))))

(event `self.K2_OnLogout`
  (params (ExitingController :type "Controller Object Reference"))
  (bind _asplayer_controller (cast `PlayerController` ExitingController))
  (`KismetArrayLibrary.Array_RemoveItem` (`self.playerControllers`) _asplayer_controller))

(fn `UserConstructionScript`)