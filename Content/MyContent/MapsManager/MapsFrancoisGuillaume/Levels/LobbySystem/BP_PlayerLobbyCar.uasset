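; BP_PlayerLobbyCar is a lobby player representation that shows a username, a ready label and a chosen material on its cube.
; Username, ready display and material changes each branch on authority, going directly to an M_ event or through an S_ event first, apparently server-to-multicast replication.
; The M_ events update two UI_Username widgets and the cube material.
; S_Ready separately sets IsReady, whose OnRep only prints the value.
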(event `S_Ready`
  (set `self.isReady` true))

(event `SetPseudo`
  (params (username :type String))
  (`/Engine/EditorBlueprintResources/ActorMacros.Switch Has Authority`
    (:`Authority`
      (`self.M_SetPseudo` username))
    (:`Remote`
      (`self.S_SetPseudo` username))))

(event `S_SetPseudo`
  (params (username :type String))
  (`self.M_SetPseudo` username))

(event `M_SetPseudo`
  (params (username :type String))
  (bind _asui_username (cast `/Game/MyContent/MapsManager/MapsFrancoisGuillaume/Levels/Menu/UI/UI_Username` (`WidgetComponent.GetWidget` (`self.WidgetUsername`))))
  (`TextBlock.SetText` (`/Game/MyContent/MapsManager/MapsFrancoisGuillaume/Levels/Menu/UI/UI_Username.txtNoName` _asui_username) (`KismetTextLibrary.Conv_StringToText` username)))

(event `AfficheReady`
  (params (ready :type Boolean))
  (`/Engine/EditorBlueprintResources/ActorMacros.Switch Has Authority`
    (:`Authority`
      (`self.M_AfficheReady` ready))
    (:`Remote`
      (`self.S_AfficheReady` ready))))

(event `S_AfficheReady`
  (params (ready :type Boolean))
  (`self.M_AfficheReady` ready))

(event `M_AfficheReady`
  (params (ready :type Boolean))
  ;[1 1 1] Affiche prêt ou pas prêt
  (bind _asui_username (cast `/Game/MyContent/MapsManager/MapsFrancoisGuillaume/Levels/Menu/UI/UI_Username` (`WidgetComponent.GetWidget` (`self.WidgetIsReady`))))
  (if ready
    (bind _txtnoname (`/Game/MyContent/MapsManager/MapsFrancoisGuillaume/Levels/Menu/UI/UI_Username.txtNoName` _asui_username))
    (`TextBlock.SetText` _txtnoname "Ready")
    (else
      (`TextBlock.SetText` _txtnoname "Not ready"))))

(event `AfficheColorPawn`
  (params (material :type "Material Object Reference"))
  (`/Engine/EditorBlueprintResources/ActorMacros.Switch Has Authority`
    (:`Authority`
      (`self.M_AfficheColorPawn` material))
    (:`Remote`
      (`self.S_AfficheColorPawn` material))))

(event `S_AfficheColorPawn`
  (params (material :type "Material Object Reference"))
  (`self.M_AfficheColorPawn` material))

(event `M_AfficheColorPawn`
  (params (material :type "Material Object Reference"))
  (`PrimitiveComponent.SetMaterial` (`self.Cube`) 0 material))

(fn `OnRep_isReady`
  (`KismetSystemLibrary.PrintString` (`KismetStringLibrary.Conv_BoolToString` (`self.isReady`))))

(fn `UserConstructionScript`)