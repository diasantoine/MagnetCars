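; Game mode for a multiplayer racing lobby, taking players from map countdown to race start.
; Tick acts as a flag-driven state machine: map countdown, race setup via GS_LobbySystem and circuit loading through BP_LoadCircuit, all-ready check, then start countdown.
; Countdowns and race start are relayed to each PC_LobbySystem.
; Login and logout maintain controller lists; CreateVehicle spawns and possesses BP_FrancoisCar at indexed player starts.
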(event `self.ReceiveTick`
  (params (DeltaSeconds :type "Float (single-precision)"))
  (if (`self.isMapSelect`)
    (if (`self.isRaceMode`)
      (if (`self.isStart`)
        _
        (elif (`self.isReady`)
          (if (<= (`self.TimeStartCounter`) 0.0)
            ;[1 0 0] Commence la course
            (set `self.isStart` true)
            (for _index (range (`KismetArrayLibrary.Array_Length` (`self.PlayerController`)))
              (bind _aspc_lobby_system (cast `/Game/MyContent/MapsManager/MapsFrancoisGuillaume/Levels/LobbySystem/PC_LobbySystem` (`GameplayStatics.GetPlayerController` _index)))
              (`/Game/MyContent/MapsManager/MapsFrancoisGuillaume/Levels/LobbySystem/PC_LobbySystem.S_DebutPartie` _aspc_lobby_system))
            (else
              ;[1 0 0] Compte à rebours
              (bind _output_get (set `self.TimeStartCounter` (- (`self.TimeStartCounter`) DeltaSeconds)))
              (for _index_2 (range (`KismetArrayLibrary.Array_Length` (`self.PlayerController`)))
                (bind _aspc_lobby_system_2 (cast `/Game/MyContent/MapsManager/MapsFrancoisGuillaume/Levels/LobbySystem/PC_LobbySystem` (`GameplayStatics.GetPlayerController` _index_2)))
                (`/Game/MyContent/MapsManager/MapsFrancoisGuillaume/Levels/LobbySystem/PC_LobbySystem.S_CompteRebours` _aspc_lobby_system_2 (`KismetMathLibrary.FTrunc` _output_get)))))
          (else
            ;[1 0 0] Vérifie si tous les joueurs sont prêts
            (set `self.isAllReadyPlayer` true)
            (for _index_3 (range (`KismetArrayLibrary.Array_Length` (`self.PlayerController`)))
              (bind _aspc_lobby_system_3 (cast `/Game/MyContent/MapsManager/MapsFrancoisGuillaume/Levels/LobbySystem/PC_LobbySystem` (`GameplayStatics.GetPlayerController` _index_3)))
              (if (not (`/Game/MyContent/MapsManager/MapsFrancoisGuillaume/Levels/LobbySystem/PC_LobbySystem.isReady` _aspc_lobby_system_3))
                (set `self.isAllReadyPlayer` false)
                (break)))
            (if (`self.isAllReadyPlayer`)
              (set `self.isReady` true)
              (set `self.TimeStartCounter` (`self.TimeStart`))))))
      (else
        ;[1 0 0] Compte à rebours
        (bind _output_get_2 (set `self.TimeMapCounter` (- (`self.TimeMapCounter`) DeltaSeconds)))
        (if (> (`self.TimeMapCounter`) 0.0)
          (for _index_4 (range (`KismetArrayLibrary.Array_Length` (`self.PlayerController`)))
            (bind _aspc_lobby_system_4 (cast `/Game/MyContent/MapsManager/MapsFrancoisGuillaume/Levels/LobbySystem/PC_LobbySystem` (`GameplayStatics.GetPlayerController` _index_4)))
            (`/Game/MyContent/MapsManager/MapsFrancoisGuillaume/Levels/LobbySystem/PC_LobbySystem.S_CompteReboursMap` _aspc_lobby_system_4 (`KismetMathLibrary.FTrunc` _output_get_2)))
          (else
            (for _index_5 (range (`KismetArrayLibrary.Array_Length` (`self.PlayerController`)))
              (bind _asgs_lobby_system (cast `/Game/MyContent/MapsManager/MapsFrancoisGuillaume/Levels/LobbySystem/GS_LobbySystem` (`GameplayStatics.GetGameState`)))
              (`/Game/MyContent/MapsManager/MapsFrancoisGuillaume/Levels/LobbySystem/GS_LobbySystem.S_SetupModeRace` _asgs_lobby_system _index_5))
            (set `self.isRaceMode` true)
            (bind _returnvalue (`GameplayStatics.GetActorOfClass` "/Game/MyContent/Blueprints/BP_LoadCircuit.BP_LoadCircuit_C" :!label _label))
            (`LoadCircuit.LoadCircuit` _returnvalue)))))))

(event `self.ReceiveBeginPlay`)

(event `S_LoadCircuit`
  (`self.M_LoadCircuit`))

(event `M_LoadCircuit`
  (goto _label))

(event `self.HandleStartingNewPlayer`
  (params (NewPlayer :type "PlayerController Object Reference"))
  (`/Engine/EditorBlueprintResources/ActorMacros.Switch Has Authority`))

(event `self.K2_PostLogin`
  (params (NewPlayer :type "PlayerController Object Reference"))
  ;[1 1 1] Quand le joueur se connecte
  (bind _asgs_lobby_system (cast `/Game/MyContent/MapsManager/MapsFrancoisGuillaume/Levels/LobbySystem/GS_LobbySystem` (`GameplayStatics.GetGameState`)))
  (`/Game/MyContent/MapsManager/MapsFrancoisGuillaume/Levels/LobbySystem/GS_LobbySystem.AddplayerController` _asgs_lobby_system NewPlayer)
  (`KismetArrayLibrary.Array_Add` (`self.PlayerController`) NewPlayer))

(event `self.K2_OnLogout`
  (params (ExitingController :type "Controller Object Reference"))
  ;[1 1 1] Quand le joueur se déconnecte
  (bind _asgs_lobby_system (cast `/Game/MyContent/MapsManager/MapsFrancoisGuillaume/Levels/LobbySystem/GS_LobbySystem` (`GameplayStatics.GetGameState`)))
  (bind _asplayer_controller (cast `PlayerController` ExitingController))
  (`/Game/MyContent/MapsManager/MapsFrancoisGuillaume/Levels/LobbySystem/GS_LobbySystem.RemovePlayerController` _asgs_lobby_system _asplayer_controller)
  (`KismetArrayLibrary.Array_RemoveItem` (`self.PlayerController`) _asplayer_controller))

(event `CreateVehicle`
  (params (nbr :type Integer))
  (bind _returnvalue (`GameplayStatics.GetPlayerController` nbr))
  (bind (_returnvalue_location _returnvalue_rotation) (`KismetMathLibrary.BreakTransform` (`self.GetTransform` (`self.K2_FindPlayerStart` _returnvalue (`KismetStringLibrary.Conv_IntToString` nbr)))))
  ;[1 0 0] Création du véhicule
  (bind _returnvalue_2 (`|SpawnActorFromClass` "/Game/MyContent/MapsManager/MapsFrancoisGuillaume/Levels/Lobby/BP_FrancoisCar.BP_FrancoisCar_C" (`KismetMathLibrary.MakeTransform` _returnvalue_location _returnvalue_rotation) "AlwaysSpawn" "OverrideRootScale" null null))
  (set `/Game/MyContent/MapsManager/MapsFrancoisGuillaume/Levels/Lobby/BP_FrancoisCar.idPlayer` nbr _returnvalue_2)
  (`Controller.Possess` _returnvalue _returnvalue_2))

(fn `UserConstructionScript`)