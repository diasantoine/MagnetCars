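; Player controller for the multiplayer lobby, per-player circuit part choice and race start.
; BeginPlay builds the lobby UI and flags the authority side as leader; Tick periodically refreshes player count, names, colors and ready labels, or in race mode repeats a limited car refresh.
; Player data is copied from GI_Player into PS_LobbySystem, then spread through S_/M_ server-to-multicast event pairs, which also carry countdowns, map choices and car enabling.
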(event `ChangeMap`
  (params (nbr :type Integer) (circuit :type "MyPartCircuit Class Reference"))
  (bind _asps_lobby_system (cast `/Game/MyContent/MapsManager/MapsFrancoisGuillaume/Levels/LobbySystem/PS_LobbySystem` (`self.PlayerState`)))
  (`/Engine/EditorBlueprintResources/ActorMacros.Switch Has Authority`
    (:`Authority`
      (bind _structure_player_id (break `/Game/MyContent/MapsManager/MapsFrancoisGuillaume/Levels/LobbySystem/Structure/Structure_Player` (`/Game/MyContent/MapsManager/MapsFrancoisGuillaume/Levels/LobbySystem/PS_LobbySystem.structure_Player` _asps_lobby_system)))
      (`self.M_ChangeMap` _structure_player_id circuit))
    (:`Remote`
      (`self.S_ChangeMap` _structure_player_id circuit))))

(event `S_ChangeMap`
  (params (nbr :type Integer) (circuit :type "MyPartCircuit Class Reference"))
  (`self.M_ChangeMap` nbr circuit))

(event `M_ChangeMap`
  (params (nbr :type Integer) (circuit :type "MyPartCircuit Class Reference"))
  (bind _returnvalue (`GameplayStatics.GetActorOfClass` "/Game/MyContent/Blueprints/BP_LoadCircuit.BP_LoadCircuit_C"))
  (`KismetSystemLibrary.PrintString` (`KismetStringLibrary.Conv_IntToString` nbr))
  (`KismetArrayLibrary.Array_Set` (`LoadCircuit.OrderPartCircuit` _returnvalue) nbr circuit))

(event `BeginChoiceMap`
  (params (id :type Integer))
  (bind _returnvalue (`|CreateWidget` "/Game/MyContent/Blueprints/WBP_ChoiceMap.WBP_ChoiceMap_C" self null id))
  (set `self.WBP ChoiceMapREF` _returnvalue)
  (`UserWidget.AddToViewport` _returnvalue 0))

(event `AfficheColorModeRace`
  (bind _asps_lobby_system (cast `/Game/MyContent/MapsManager/MapsFrancoisGuillaume/Levels/LobbySystem/PS_LobbySystem` (`Controller.PlayerState` (`GameplayStatics.GetPlayerController` 0))))
  (bind _ascharacter_car_cube (cast `/Game/MyContent/MapsManager/MapsFrancoisGuillaume/Levels/Lobby/Character_CarCube` (`self.K2_GetPawn` (`GameplayStatics.GetPlayerController` 0))))
  (bind (_structure_player_id _structure_player_username _structure_player_material) (break `/Game/MyContent/MapsManager/MapsFrancoisGuillaume/Levels/LobbySystem/Structure/Structure_Player` (`/Game/MyContent/MapsManager/MapsFrancoisGuillaume/Levels/LobbySystem/PS_LobbySystem.structure_Player` _asps_lobby_system)))
  (`self.S_AfficheColorModeRace` _ascharacter_car_cube _structure_player_material))

(event `S_AfficheColorModeRace`
  (params (car :type "/Game/MyContent/MapsManager/MapsFrancoisGuillaume/Levels/Lobby/Character_CarCube Object Reference") (material :type "Material Object Reference"))
  (`self.M_AfficheColorModeRace` car material))

(event `M_AfficheColorModeRace`
  (params (car :type "/Game/MyContent/MapsManager/MapsFrancoisGuillaume/Levels/Lobby/Character_CarCube Object Reference") (material :type "Material Object Reference"))
  (`PrimitiveComponent.SetMaterial` (`/Game/MyContent/MapsManager/MapsFrancoisGuillaume/Levels/Lobby/Character_CarCube.Cube` car) 0 material))

(event `S_AffichePseudoModeRace`
  (params (username :type String) (car :type "/Game/MyContent/MapsManager/MapsFrancoisGuillaume/Levels/Lobby/Character_CarCube Object Reference"))
  (`self.M_AffichePseudoModeRace` username car))

(event `AffichePseudoModeRace`
  (`self.InitStruct`)
  (bind _asps_lobby_system (cast `/Game/MyContent/MapsManager/MapsFrancoisGuillaume/Levels/LobbySystem/PS_LobbySystem` (`Controller.PlayerState` (`GameplayStatics.GetPlayerController` 0))))
  (bind _ascharacter_car_cube (cast `/Game/MyContent/MapsManager/MapsFrancoisGuillaume/Levels/Lobby/Character_CarCube` (`self.K2_GetPawn` (`GameplayStatics.GetPlayerController` 0))))
  (bind (_structure_player_id _structure_player_username) (break `/Game/MyContent/MapsManager/MapsFrancoisGuillaume/Levels/LobbySystem/Structure/Structure_Player` (`/Game/MyContent/MapsManager/MapsFrancoisGuillaume/Levels/LobbySystem/PS_LobbySystem.structure_Player` _asps_lobby_system)))
  (`self.S_AffichePseudoModeRace` _structure_player_username _ascharacter_car_cube))

(event `M_AffichePseudoModeRace`
  (params (username :type String) (car :type "/Game/MyContent/MapsManager/MapsFrancoisGuillaume/Levels/Lobby/Character_CarCube Object Reference"))
  (bind _asui_username (cast `/Game/MyContent/MapsManager/MapsFrancoisGuillaume/Levels/Menu/UI/UI_Username` (`WidgetComponent.GetWidget` (`/Game/MyContent/MapsManager/MapsFrancoisGuillaume/Levels/Lobby/Character_CarCube.WidgetUsername` car))))
  (`TextBlock.SetText` (`/Game/MyContent/MapsManager/MapsFrancoisGuillaume/Levels/Menu/UI/UI_Username.txtNoName` _asui_username) (`KismetTextLibrary.Conv_StringToText` username)))

(event `DisplayNumPlayer`
  (params (nbrPlayer :type Integer) (nbrMaxPlayer :type Integer))
  ;[1 1 1] Affiche le nombre de joueurs
  (`TextBlock.SetText` (`/Game/MyContent/MapsManager/MapsFrancoisGuillaume/Levels/Lobby/UI_Lobby.txtNbrJoueur` (`self.UI_LobbyREF`)) (`KismetTextLibrary.Conv_StringToText` (`KismetStringLibrary.Concat_StrStr` "Players  " (`KismetStringLibrary.Conv_IntToString` nbrPlayer) " / " (`KismetStringLibrary.Conv_IntToString` nbrMaxPlayer)))))

(event `RefreshStatutPlayerRaceMode`
  ;[1 1 1] Actualise le statut du joueur
  (`self.DisplayNumPlayer` (`KismetArrayLibrary.Array_Length` (`GameStateBase.PlayerArray` (`GameplayStatics.GetGameState`))) 4)
  (`self.AffichePseudoModeRace`)
  (`self.AfficheColorModeRace`))

(event `M_DebutPartie`
  ;[1 1 1] Début de partie
  ;;[1 0 0] Autorise le joueur à bouger
  (bind _asbp_francois_car (cast `/Game/MyContent/MapsManager/MapsFrancoisGuillaume/Levels/Lobby/BP_FrancoisCar` (`self.K2_GetPawn` (`GameplayStatics.GetPlayerController` 0))))
  (set `/Game/MyContent/MapsManager/MapsFrancoisGuillaume/Levels/Lobby/BP_FrancoisCar.isEnable` true _asbp_francois_car)
  ;;[1 0 0] Désactive l'UI compte à rebours
  (`TextBlock.SetText` (`/Game/MyContent/MapsManager/MapsFrancoisGuillaume/Levels/Lobby/UI_Lobby.TxtCountdown` (`self.UI_LobbyREF`)) ""))

(event `S_DebutPartie`
  ;[1 1 1] Début de partie
  (`self.M_DebutPartie`))

(event `S_CompteReboursMap`
  (params (second :type Integer))
  ;[1 1 1] Affichage du compte à rebours
  (`self.M_CompteReboursMap` second))

(event `M_CompteReboursMap`
  (params (second :type Integer))
  ;[1 1 1] Affichage du compte à rebours
  (`TextBlock.SetText` (`/Game/MyContent/Blueprints/WBP_ChoiceMap.TxtCountdown` (`self.WBP ChoiceMapREF`)) (`KismetTextLibrary.Conv_IntToText` second)))

(event `S_CompteRebours`
  (params (second :type Integer))
  ;[1 1 1] Affichage du compte à rebours
  (`self.M_CompteRebours` second))

(event `M_CompteRebours`
  (params (second :type Integer))
  ;[1 1 1] Affichage du compte à rebours
  (`TextBlock.SetText` (`/Game/MyContent/MapsManager/MapsFrancoisGuillaume/Levels/Lobby/UI_Lobby.TxtCountdown` (`self.UI_LobbyREF`)) (`KismetTextLibrary.Conv_StringToText` (`KismetStringLibrary.Conv_IntToString` second))))

(event `BeginModeRace`
  (bind _texttest (`/Game/MyContent/MapsManager/MapsFrancoisGuillaume/Levels/Lobby/UI_Lobby.TextTest` (`self.UI_LobbyREF`)))
  (set `self.bShowMouseCursor` false)
  (bind _returnvalue (`|CreateWidget` "/Game/MyContent/MapsManager/MapsFrancoisGuillaume/Levels/Lobby/UI_Lobby.UI_Lobby_C" self))
  (set `self.UI_LobbyREF` _returnvalue)
  (`UserWidget.AddToViewport` _returnvalue 0)
  (`AdvancedSessionsLibrary.GetSessionSettings`
    (:`OnSuccess`
      (`TextBlock.SetText` _texttest "oui"))
    (:`OnFailure`
      (`TextBlock.SetText` _texttest "non"))))

(event `self.ReceiveTick`
  (params (DeltaSeconds :type "Float (single-precision)"))
  (if (`self.isRaceMode`)
    ;[1 1 1] Event Tick
    (if (`self.isNotMapChoice`)
      (if (not (`self.isReady`))
        ;;[1 0 0] Laisse le temps de se charger
        (if (>= (`self.TimePcCounter`) (`self.TimePC`))
          (set `self.TimePcCounter` 0.0)
          (`self.RefreshStatutPlayerRaceMode`)
          (set `self.nbrActualisation` (- (`self.nbrActualisation`) 1))
          (if (<= (`self.nbrActualisation`) 0)
            (set `self.isReady` true))
          (else
            (set `self.TimePcCounter` (+ (`self.TimePcCounter`) DeltaSeconds))))))
    (else
      ;[1 1 1] Actualise les statuts des joueurs
      (if (>= (`self.TimePcCounter`) (`self.TimePC`))
        (set `self.TimePcCounter` 0.0)
        (`self.RefreshStatutPlayer`)
        (else
          (set `self.TimePcCounter` (+ (`self.TimePcCounter`) DeltaSeconds)))))))

(event `InitController`
  (params (id :type Integer))
  ;[1 1 1] Initialisation du joueur pour déterminer si c'est l'hote du serveur ou le client
  (bind _asps_lobby_system (cast `/Game/MyContent/MapsManager/MapsFrancoisGuillaume/Levels/LobbySystem/PS_LobbySystem` (`GameplayStatics.GetPlayerState` 0)))
  (if (< id 1)
    (set `/Game/MyContent/MapsManager/MapsFrancoisGuillaume/Levels/LobbySystem/PS_LobbySystem.isLeader` true _asps_lobby_system)
    (else
      (set `/Game/MyContent/MapsManager/MapsFrancoisGuillaume/Levels/LobbySystem/PS_LobbySystem.isLeader` false _asps_lobby_system))))

(event `self.ReceiveBeginPlay`
  (bind _ui_ref (`self.UI_REF`))
  ;[1 1 1] Affiche l'UI
  (bind _returnvalue (`|CreateWidget` "/Game/MyContent/MapsManager/MapsFrancoisGuillaume/Levels/LobbySystem/UI_LobbySystem.UI_LobbySystem_C" self))
  (bind _output_get (set `self.UI_REF` _returnvalue))
  (`UserWidget.AddToViewport` _output_get 0)
  (`self.InitStructState`)
  ;[1 1 1] Initialise l'UI
  (`/Engine/EditorBlueprintResources/ActorMacros.Switch Has Authority`
    (:`Authority`
      (`Widget.SetVisibility` (`/Game/MyContent/MapsManager/MapsFrancoisGuillaume/Levels/LobbySystem/UI_LobbySystem.Button_Start` _ui_ref) "Visible")
      (`Widget.SetVisibility` (`/Game/MyContent/MapsManager/MapsFrancoisGuillaume/Levels/LobbySystem/UI_LobbySystem.Button_Ready` _ui_ref) "Hidden")
      (`Widget.SetVisibility` (`/Game/MyContent/MapsManager/MapsFrancoisGuillaume/Levels/LobbySystem/UI_LobbySystem.Button_NotReady` _ui_ref) "Hidden")
      (`self.InitController` 0))
    (:`Remote`
      (`self.InitController` 1))))

(event `S_SetupIsready`
  (params (isReady :type Boolean))
  ;[1 1 1] Met le joueur prêt ou pas
  (`self.M_SetupIsReady` isReady))

(event `M_SetupIsReady`
  (params (isReady :type Boolean))
  ;[1 1 1] Met le joueur prêt ou pas
  (bind _asps_lobby_system (cast `/Game/MyContent/MapsManager/MapsFrancoisGuillaume/Levels/LobbySystem/PS_LobbySystem` (`self.PlayerState`)))
  (set `/Game/MyContent/MapsManager/MapsFrancoisGuillaume/Levels/LobbySystem/PS_LobbySystem.isReady` isReady _asps_lobby_system))

(event `CustomEvent_2`
  (`KismetSystemLibrary.PrintString` "Hello"))

(event `Key|A`
  (params (Key :type "Key Structure")))

(event `RefreshStatutPlayer`
  ;[1 1 1] Affiche le nombre de joueurs
  (`self.GetNbrPlayerUI`)
  ;[1 1 1] Affiche le pseudo du joueur que l'on controle en rouge
  (`self.SetColorForMainUsername`)
  ;[1 1 1] Affiche le leader en jaune
  (`self.AfficheLeLeader`)
  ;[1 1 1] Vérifie si le joueur est le serveur ou le client
  (bind _asps_lobby_system (cast `/Game/MyContent/MapsManager/MapsFrancoisGuillaume/Levels/LobbySystem/PS_LobbySystem` (`Controller.PlayerState` (`GameplayStatics.GetPlayerController` 0))))
  (if (`/Game/MyContent/MapsManager/MapsFrancoisGuillaume/Levels/LobbySystem/PS_LobbySystem.isLeader` _asps_lobby_system)
    (`self.AffichePseudo`)
    (`self.AfficheColor`)
    (else
      (`self.AfficheReady`)
      (`self.AffichePseudo`)
      (`self.AfficheColor`))))

(event `AfficheReady`
  ;[1 1 1] Initialise les variables avant de les multicaster
  (bind _asps_lobby_system (cast `/Game/MyContent/MapsManager/MapsFrancoisGuillaume/Levels/LobbySystem/PS_LobbySystem` (`Controller.PlayerState` (`GameplayStatics.GetPlayerController` 0))))
  (bind _asbp_player_lobby_car (cast `/Game/MyContent/MapsManager/MapsFrancoisGuillaume/Levels/LobbySystem/BP_PlayerLobbyCar` (`/Game/MyContent/MapsManager/MapsFrancoisGuillaume/Levels/LobbySystem/PS_LobbySystem.actorPlayer` _asps_lobby_system)))
  (`self.S_AfficheReady` _asbp_player_lobby_car (`/Game/MyContent/MapsManager/MapsFrancoisGuillaume/Levels/LobbySystem/PS_LobbySystem.isReady` _asps_lobby_system)))

(event `S_AfficheReady`
  (params (ActorPlayer :type "/Game/MyContent/MapsManager/MapsFrancoisGuillaume/Levels/LobbySystem/BP_PlayerLobbyCar Object Reference") (isReady :type Boolean))
  (`self.M_AfficheReady` ActorPlayer isReady))

(event `M_AfficheReady`
  (params (ActorPlayer :type "/Game/MyContent/MapsManager/MapsFrancoisGuillaume/Levels/LobbySystem/BP_PlayerLobbyCar Object Reference") (isReady :type Boolean))
  ;[1 1 1] Affiche prêt ou pas prêt
  (bind _asui_username (cast `/Game/MyContent/MapsManager/MapsFrancoisGuillaume/Levels/Menu/UI/UI_Username` (`WidgetComponent.GetWidget` (`/Game/MyContent/MapsManager/MapsFrancoisGuillaume/Levels/LobbySystem/BP_PlayerLobbyCar.WidgetIsReady` ActorPlayer))))
  (if isReady
    (bind _txtnoname (`/Game/MyContent/MapsManager/MapsFrancoisGuillaume/Levels/Menu/UI/UI_Username.txtNoName` _asui_username))
    (`TextBlock.SetText` _txtnoname "Ready")
    (else
      (`TextBlock.SetText` _txtnoname "Not ready"))))

(event `AffichePseudo`
  (bind _returnvalue (`GameplayStatics.GetPlayerController` 0))
  (bind _playername (`AdvancedSessionsLibrary.GetPlayerName` _returnvalue))
  ;[1 1 1] Initialise les variables avant de les multicaster
  (`self.InitStructState`)
  (bind _asps_lobby_system (cast `/Game/MyContent/MapsManager/MapsFrancoisGuillaume/Levels/LobbySystem/PS_LobbySystem` (`Controller.PlayerState` _returnvalue)))
  (bind _asbp_player_lobby_car (cast `/Game/MyContent/MapsManager/MapsFrancoisGuillaume/Levels/LobbySystem/BP_PlayerLobbyCar` (`/Game/MyContent/MapsManager/MapsFrancoisGuillaume/Levels/LobbySystem/PS_LobbySystem.actorPlayer` _asps_lobby_system)))
  (bind _asgi_player (cast `/Game/MyContent/MapsManager/MapsFrancoisGuillaume/Levels/Menu/GI_Player` (`GameplayStatics.GetGameInstance`)))
  (`/Engine/EditorBlueprintResources/ActorMacros.Switch Has Authority`
    (:`Authority`
      (`self.M_AffichePseudo` _asbp_player_lobby_car _playername))
    (:`Remote`
      (`self.S_AffichePseudo` _asbp_player_lobby_car _playername))))

(event `S_AffichePseudo`
  (params (actorPlayer :type "/Game/MyContent/MapsManager/MapsFrancoisGuillaume/Levels/LobbySystem/BP_PlayerLobbyCar Object Reference") (username :type String))
  (`self.M_AffichePseudo` actorPlayer username))

(event `M_AffichePseudo`
  (params (actorPlayer :type "/Game/MyContent/MapsManager/MapsFrancoisGuillaume/Levels/LobbySystem/BP_PlayerLobbyCar Object Reference") (username :type String))
  (bind _asui_username (cast `/Game/MyContent/MapsManager/MapsFrancoisGuillaume/Levels/Menu/UI/UI_Username` (`WidgetComponent.GetWidget` (`/Game/MyContent/MapsManager/MapsFrancoisGuillaume/Levels/LobbySystem/BP_PlayerLobbyCar.WidgetUsername` actorPlayer))))
  (`TextBlock.SetText` (`/Game/MyContent/MapsManager/MapsFrancoisGuillaume/Levels/Menu/UI/UI_Username.txtNoName` _asui_username) (`KismetTextLibrary.Conv_StringToText` username)))

(event `AfficheColor`
  (bind _asps_lobby_system (cast `/Game/MyContent/MapsManager/MapsFrancoisGuillaume/Levels/LobbySystem/PS_LobbySystem` (`Controller.PlayerState` (`GameplayStatics.GetPlayerController` 0))))
  (bind _asbp_player_lobby_car (cast `/Game/MyContent/MapsManager/MapsFrancoisGuillaume/Levels/LobbySystem/BP_PlayerLobbyCar` (`/Game/MyContent/MapsManager/MapsFrancoisGuillaume/Levels/LobbySystem/PS_LobbySystem.actorPlayer` _asps_lobby_system)))
  (bind (_structure_player_id _structure_player_username _structure_player_material) (break `/Game/MyContent/MapsManager/MapsFrancoisGuillaume/Levels/LobbySystem/Structure/Structure_Player` (`/Game/MyContent/MapsManager/MapsFrancoisGuillaume/Levels/LobbySystem/PS_LobbySystem.structure_Player` _asps_lobby_system)))
  (`self.S_AfficheColor` _asbp_player_lobby_car _structure_player_material))

(event `S_AfficheColor`
  (params (ActorPlayer :type "/Game/MyContent/MapsManager/MapsFrancoisGuillaume/Levels/LobbySystem/BP_PlayerLobbyCar Object Reference") (Color :type "Material Object Reference"))
  (`self.M_AfficheColor` ActorPlayer Color))

(event `M_AfficheColor`
  (params (ActorPlayer :type "/Game/MyContent/MapsManager/MapsFrancoisGuillaume/Levels/LobbySystem/BP_PlayerLobbyCar Object Reference") (Color :type "Material Object Reference"))
  (`PrimitiveComponent.SetMaterial` (`/Game/MyContent/MapsManager/MapsFrancoisGuillaume/Levels/LobbySystem/BP_PlayerLobbyCar.Cube` ActorPlayer) 0 Color))

(fn `AfficheLeLeader`
  ;[1 1 1] Affiche qui est l'hote du serveur
  (for _index (range (`GameplayStatics.GetNumPlayerStates`))
    (bind _asps_lobby_system (cast `/Game/MyContent/MapsManager/MapsFrancoisGuillaume/Levels/LobbySystem/PS_LobbySystem` (`GameplayStatics.GetPlayerState` _index)))
    (bind _structure_player_id (break `/Game/MyContent/MapsManager/MapsFrancoisGuillaume/Levels/LobbySystem/Structure/Structure_Player` (`/Game/MyContent/MapsManager/MapsFrancoisGuillaume/Levels/LobbySystem/PS_LobbySystem.structure_Player` _asps_lobby_system)))
    (if (== _structure_player_id 0)
      (bind _asbp_player_lobby_car (cast `/Game/MyContent/MapsManager/MapsFrancoisGuillaume/Levels/LobbySystem/BP_PlayerLobbyCar` (`/Game/MyContent/MapsManager/MapsFrancoisGuillaume/Levels/LobbySystem/PS_LobbySystem.actorPlayer` _asps_lobby_system)))
      (bind _asui_username (cast `/Game/MyContent/MapsManager/MapsFrancoisGuillaume/Levels/Menu/UI/UI_Username` (`WidgetComponent.GetWidget` (`/Game/MyContent/MapsManager/MapsFrancoisGuillaume/Levels/LobbySystem/BP_PlayerLobbyCar.WidgetIsReady` _asbp_player_lobby_car))))
      (bind _txtnoname (`/Game/MyContent/MapsManager/MapsFrancoisGuillaume/Levels/Menu/UI/UI_Username.txtNoName` _asui_username))
      (`TextBlock.SetText` _txtnoname "Leader")
      (`TextBlock.SetColorAndOpacity` _txtnoname (make `SlateColor` (struct :`R` 0.708135 :`G` 1.0 :`A` 1.0))))))

(fn `GetNbrPlayerUI`
  ;[1 1 1] Affiche le nombre de joueurs
  (`TextBlock.SetText` (`/Game/MyContent/MapsManager/MapsFrancoisGuillaume/Levels/LobbySystem/UI_LobbySystem.TxtNbrPlayer` (`self.UI_REF`)) (`KismetTextLibrary.Conv_IntToText` (`KismetArrayLibrary.Array_Length` (`GameStateBase.PlayerArray` (`GameplayStatics.GetGameState`))))))

(fn `InitStruct`
  (bind _asgi_player (cast `/Game/MyContent/MapsManager/MapsFrancoisGuillaume/Levels/Menu/GI_Player` (`GameplayStatics.GetGameInstance`)))
  (bind _asps_lobby_system (cast `/Game/MyContent/MapsManager/MapsFrancoisGuillaume/Levels/LobbySystem/PS_LobbySystem` (`Controller.PlayerState` (`GameplayStatics.GetPlayerController` 0))))
  (bind _structure_player_id (break `/Game/MyContent/MapsManager/MapsFrancoisGuillaume/Levels/LobbySystem/Structure/Structure_Player` (`/Game/MyContent/MapsManager/MapsFrancoisGuillaume/Levels/LobbySystem/PS_LobbySystem.structure_Player` _asps_lobby_system)))
  (bind (_structure_player_id_2 _structure_player_username _structure_player_material) (break `/Game/MyContent/MapsManager/MapsFrancoisGuillaume/Levels/LobbySystem/Structure/Structure_Player` (`/Game/MyContent/MapsManager/MapsFrancoisGuillaume/Levels/Menu/GI_Player.structure_Player` _asgi_player)))
  (set `/Game/MyContent/MapsManager/MapsFrancoisGuillaume/Levels/LobbySystem/PS_LobbySystem.structure_Player` (make `/Game/MyContent/MapsManager/MapsFrancoisGuillaume/Levels/LobbySystem/Structure/Structure_Player` _structure_player_id _structure_player_username _structure_player_material) _asps_lobby_system))

(fn `InitStructState`
  ;[1 1 1] Initialisation des données qui sont stockées pour les ditribuer
  (bind _asgi_player (cast `/Game/MyContent/MapsManager/MapsFrancoisGuillaume/Levels/Menu/GI_Player` (`GameplayStatics.GetGameInstance`)))
  (bind _asps_lobby_system (cast `/Game/MyContent/MapsManager/MapsFrancoisGuillaume/Levels/LobbySystem/PS_LobbySystem` (`Controller.PlayerState` (`GameplayStatics.GetPlayerController` 0))))
  (bind _structure_player_id (break `/Game/MyContent/MapsManager/MapsFrancoisGuillaume/Levels/LobbySystem/Structure/Structure_Player` (`/Game/MyContent/MapsManager/MapsFrancoisGuillaume/Levels/LobbySystem/PS_LobbySystem.structure_Player` _asps_lobby_system)))
  (bind (_structure_player_id_2 _structure_player_username _structure_player_material) (break `/Game/MyContent/MapsManager/MapsFrancoisGuillaume/Levels/LobbySystem/Structure/Structure_Player` (`/Game/MyContent/MapsManager/MapsFrancoisGuillaume/Levels/Menu/GI_Player.structure_Player` _asgi_player)))
  (set `/Game/MyContent/MapsManager/MapsFrancoisGuillaume/Levels/LobbySystem/PS_LobbySystem.structure_Player` (make `/Game/MyContent/MapsManager/MapsFrancoisGuillaume/Levels/LobbySystem/Structure/Structure_Player` _structure_player_id _structure_player_username _structure_player_material) _asps_lobby_system))

(fn `SetColorForMainUsername`
  ;[1 1 1] Affiche le pseudo en rouge le pseudo du joueur que l'on controle
  (bind _asps_lobby_system (cast `/Game/MyContent/MapsManager/MapsFrancoisGuillaume/Levels/LobbySystem/PS_LobbySystem` (`Controller.PlayerState` (`GameplayStatics.GetPlayerController` 0))))
  (bind _asbp_player_lobby_car (cast `/Game/MyContent/MapsManager/MapsFrancoisGuillaume/Levels/LobbySystem/BP_PlayerLobbyCar` (`/Game/MyContent/MapsManager/MapsFrancoisGuillaume/Levels/LobbySystem/PS_LobbySystem.actorPlayer` _asps_lobby_system)))
  (bind _asui_username (cast `/Game/MyContent/MapsManager/MapsFrancoisGuillaume/Levels/Menu/UI/UI_Username` (`WidgetComponent.GetWidget` (`/Game/MyContent/MapsManager/MapsFrancoisGuillaume/Levels/LobbySystem/BP_PlayerLobbyCar.WidgetUsername` _asbp_player_lobby_car))))
  (`TextBlock.SetColorAndOpacity` (`/Game/MyContent/MapsManager/MapsFrancoisGuillaume/Levels/Menu/UI/UI_Username.txtNoName` _asui_username) (make `SlateColor` (struct :`R` 1.0 :`G` 0.025 :`A` 1.0))))

(fn `UserConstructionScript`)