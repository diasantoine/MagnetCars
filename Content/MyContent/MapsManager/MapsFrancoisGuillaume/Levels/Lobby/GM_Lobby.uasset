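; GM_Lobby is the lobby game mode that spawns joining players and starts the game once all are ready.
; Each new player possesses a Character_CarCube spawned at a PlayerStart looked up by join index, and is tracked in PlayerControllers until logout.
; Tick polls each PC_Lobby's IsReady, then runs a countdown, sending remaining seconds through SCompteRebours and calling SDebutPartie at zero.
; Once the countdown begins, readiness is not rechecked.
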(event `self.ReceiveBeginPlay`)

(event `self.ReceiveTick`
  (params (DeltaSeconds :type "Float (single-precision)"))
  (if (`self.isStart`)
    _
    (elif (`self.isReady`)
      (if (<= (`self.TimeStartCounter`) 0.0)
        (set `self.isStart` true)
        (for _index (range (`KismetArrayLibrary.Array_Length` (`self.PlayerControllers`)))
          (bind _aspc_lobby (cast `/Game/MyContent/MapsManager/MapsFrancoisGuillaume/Levels/Lobby/PC_Lobby` (`GameplayStatics.GetPlayerController` _index)))
          (`/Game/MyContent/MapsManager/MapsFrancoisGuillaume/Levels/Lobby/PC_Lobby.S_DebutPartie` _aspc_lobby))
        (else
          (bind _output_get (set `self.TimeStartCounter` (- (`self.TimeStartCounter`) DeltaSeconds)))
          (for _index_2 (range (`KismetArrayLibrary.Array_Length` (`self.PlayerControllers`)))
            (bind _aspc_lobby_2 (cast `/Game/MyContent/MapsManager/MapsFrancoisGuillaume/Levels/Lobby/PC_Lobby` (`GameplayStatics.GetPlayerController` _index_2)))
            (`/Game/MyContent/MapsManager/MapsFrancoisGuillaume/Levels/Lobby/PC_Lobby.S_CompteRebours` _aspc_lobby_2 (`KismetMathLibrary.FTrunc` _output_get)))))
      (else
        ;[1 1 1] Vérifie si tous les joueurs sont prêts
        (set `self.isAllReadyPlayer` true)
        (for _index_3 (range (`KismetArrayLibrary.Array_Length` (`self.PlayerControllers`)))
          (bind _aspc_lobby_3 (cast `/Game/MyContent/MapsManager/MapsFrancoisGuillaume/Levels/Lobby/PC_Lobby` (`GameplayStatics.GetPlayerController` _index_3)))
          (if (not (`/Game/MyContent/MapsManager/MapsFrancoisGuillaume/Levels/Lobby/PC_Lobby.isReady` _aspc_lobby_3))
            (set `self.isAllReadyPlayer` false)
            (break)))
        (if (`self.isAllReadyPlayer`)
          (set `self.isReady` true)
          (set `self.TimeStartCounter` (`self.TimeStart`)))))))

(event `self.K2_PostLogin`
  (params (NewPlayer :type "PlayerController Object Reference")))

(event `self.HandleStartingNewPlayer`
  (params (NewPlayer :type "PlayerController Object Reference"))
  ;[1 1 1] Connexion du joueur
  (bind _returnvalue (`KismetArrayLibrary.Array_Add` (`self.PlayerControllers`) NewPlayer))
  (bind (_returnvalue_location _returnvalue_rotation) (`KismetMathLibrary.BreakTransform` (`self.GetTransform` (`self.K2_FindPlayerStart` NewPlayer (`KismetStringLibrary.Conv_IntToString` _returnvalue)))))
  (bind _returnvalue_2 (`|SpawnActorFromClass` "/Game/MyContent/MapsManager/MapsFrancoisGuillaume/Levels/Lobby/Character_CarCube.Character_CarCube_C" (`KismetMathLibrary.MakeTransform` _returnvalue_location _returnvalue_rotation) "AlwaysSpawn" "OverrideRootScale" null "No name" null))
  (`Controller.Possess` NewPlayer _returnvalue_2))

(event `self.K2_OnLogout`
  (params (ExitingController :type "Controller Object Reference"))
  ;[1 1 1] Deconnexion du joueur
  (bind _asplayer_controller (cast `PlayerController` ExitingController))
  (`KismetArrayLibrary.Array_RemoveItem` (`self.PlayerControllers`) _asplayer_controller))

(fn `OnRep_playerControllers`)

(fn `UserConstructionScript`)