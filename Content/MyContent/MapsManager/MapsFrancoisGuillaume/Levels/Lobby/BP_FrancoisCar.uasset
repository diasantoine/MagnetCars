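; BP_FrancoisCar is a player-driven car Blueprint in the Lobby folder, with movement, drift, gravity change and respawn inputs.
; Inputs call movement functions locally, mostly gated by IsEnable; their server/multicast relays are left unwired or unfinished.
; Each tick, the controlling instance packs transform and velocity into StructCarStat, then triggers server or multicast events.
; Non-controlling instances snap actor, collision and mesh to that state, without interpolation.
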(event `S_LocAndRot`
  (`self.M_LocAndRot`))

(event `M_LocAndRot`
  (bind (_structcarstat_position _structcarstat_rotation _structcarstat_velocity _structcarstat_rotationcollision _structcarstat_rotationmesh) (break `/Game/MyContent/MapsManager/MapsFrancoisGuillaume/Levels/Lobby/StructStatCar` (`self.structCarStat`)))
  (if (not (`self.IsLocallyControlled`))
    (`self.K2_SetActorLocationAndRotation` _structcarstat_position _structcarstat_rotation false true)
    (`SceneComponent.K2_SetRelativeRotation` (`self.CarCollision`) _structcarstat_rotationcollision false false)
    (`SceneComponent.K2_SetRelativeRotation` (`self.SkeletalMesh`) _structcarstat_rotationmesh false false)))

(event `InputAxis|LookUp`
  (params (AxisValue :type "Float (single-precision)"))
  (if (`self.isEnable`)
    (`self.UpMovement` AxisValue)))

(event `InputAction|Respawn`
  (params (Key :type "Key Structure"))
  (:`Pressed`
    (if (`self.isEnable`)
      (`self.CarRespawn`))))

(event `S_Respawn`
  (`self.M_Respawn`))

(event `M_Respawn`)

(event `InputAction|ResetScene`
  (params (Key :type "Key Structure"))
  (:`Pressed`
    (`KismetSystemLibrary.PrintString` "Hello")))

(event `InputAction|ChangeGravity`
  (params (Key :type "Key Structure"))
  (:`Pressed`
    (if (`self.isEnable`)
      (`self.CarGravity` :!label _label))))

(event `S_CarGravity`
  (`self.M_CarGravity`))

(event `M_CarGravity`
  (goto _label))

(event `InputAxis|LeftLean`
  (params (AxisValue :type "Float (single-precision)"))
  (if (`self.isEnable`)
    (`self.CarDrift` AxisValue)
    (else
      (`self.CarDrift` 0.0))))

(event `M_CarDrift`
  (params (axis :type "Float (double-precision)"))
  (`self.CarDrift` (stale `InputAxis|RightLean` AxisValue) :!label _label_2))

(event `S_CarDrift`
  (params (axis :type "Float (double-precision)"))
  (`self.M_CarDrift` axis))

(event `InputAxis|RightLean`
  (params (AxisValue :type "Float (single-precision)"))
  (if (`self.isEnable`)
    (goto _label_2)
    (else
      (`self.CarDrift` 0.0))))

(event `InputAxis|Right`
  (params (AxisValue :type "Float (single-precision)"))
  (if (`self.isEnable`)
    (`self.RightMovement` AxisValue :!label _label_3)
    (else
      (`self.RightMovement` 0.0))))

(event `S_Right`
  (params (axis :type "Float (double-precision)"))
  (`self.M_Right` axis))

(event `M_Right`
  (params (axis :type "Float (double-precision)"))
  (goto _label_3))

(event `S_Forward`
  (params (axis :type "Float (double-precision)"))
  (`self.M_Forward` axis))

(event `M_Forward`
  (params (axis :type "Float (double-precision)"))
  (`self.ForwardMovement` (stale `InputAxis|Forward` AxisValue) :!label _label_4))

(event `InputAxis|Forward`
  (params (AxisValue :type "Float (single-precision)"))
  (if (`self.isEnable`)
    (set `self.inputForward` AxisValue)
    (goto _label_4)
    (else
      (`self.ForwardMovement` 0.0))))

(event `self.ReceiveBeginPlay`
  (set `self.TemporaryScene` (`self.Scene`))
  (`parent.ReceiveBeginPlay`))

(event `CustomEvent_0`
  (params (NewParam :type "/Game/MyContent/MapsManager/MapsFrancoisGuillaume/Levels/Lobby/StructStatCar Structure"))
  (set `self.structCarStat` NewParam))

(event `self.ReceiveTick`
  (params (DeltaSeconds :type "Float (single-precision)"))
  (`self.MovementManager`)
  (`parent.ReceiveTick` DeltaSeconds))

(fn `MovementManager`
  (if (`self.IsLocallyControlled`)
    (bind _output_get (set `self.structCarStat` (make `/Game/MyContent/MapsManager/MapsFrancoisGuillaume/Levels/Lobby/StructStatCar` (`self.K2_GetActorLocation`) (`self.GetControlRotation`) (`self.GetVelocity`) (`SceneComponent.RelativeRotation` (`self.CarCollision`)) (`SceneComponent.RelativeRotation` (`self.Scene`)))))
    (`self.CustomEvent_0` _output_get)
    (`/Engine/EditorBlueprintResources/ActorMacros.Switch Has Authority`
      (:`Authority`
        (`self.M_LocAndRot`))
      (:`Remote`
        (`self.S_LocAndRot`)))))

(fn `UserConstructionScript`)