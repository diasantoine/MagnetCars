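; Player controller for the multiplayer car lobby, creating the speed and lobby widgets and showing player count, names and car colours.
; Tick runs a limited number of timed refreshes, copying GameInstance username and material into PlayerState, then applying them to the controlled car.
; Paired S_/M_ events, named as server-to-multicast relays, pass on names, colours, the countdown and the game start that enables car movement.
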(event `self.ReceiveBeginPlay`
  (bind _returnvalue (`|CreateWidget` "/Game/MyContent/Blueprints/WBP_Speed.WBP_Speed_C" self))
  (bind _output_get (set `self.VehicleHud` _returnvalue))
  (`UserWidget.AddToViewport` _output_get 0)
  (bind _returnvalue_2 (`|CreateWidget` "/Game/MyContent/MapsManager/MapsFrancoisGuillaume/Levels/Lobby/UI_Lobby.UI_Lobby_C" self))
  (set `self.UI_LobbyREF` _returnvalue_2)
  (`UserWidget.AddToViewport` _returnvalue_2 0))

(event `self.ReceiveTick`
  (params (DeltaSeconds :type "Float (single-precision)"))
  (if (`self.isReady`)
    _
    (elif (>= (`self.TimePcCounter`) (`self.TimePC`))
      (set `self.TimePcCounter` 0.0)
      (`self.RefreshStatutPlayer`)
      (set `self.nbrActualisation` (- (`self.nbrActualisation`) 1))
      (if (<= (`self.nbrActualisation`) 0)
        (set `self.isReady` true))
      (else
        (set `self.TimePcCounter` (+ (`self.TimePcCounter`) DeltaSeconds))))))

(event `CustomEvent_0`
  (params (NewParam :type String))
  (`KismetSystemLibrary.PrintString` NewParam))

(event `Key|SpaceBar`
  (params (Key :type "Key Structure"))
  (:`Pressed`
    (`self.CustomEvent_0` (`AdvancedSessionsLibrary.GetPlayerName` (`GameplayStatics.GetPlayerController` 0)))))

(event `RefreshStatutPlayer`
  (`self.DisplayNumPlayer` (`KismetArrayLibrary.Array_Length` (`GameStateBase.PlayerArray` (`GameplayStatics.GetGameState`))) 4)
  (`self.AffichePseudo`)
  (`self.AfficheColor`))

(event `DisplayNumPlayer`
  (params (nbrPlayer :type Integer) (nbrMaxPlayer :type Integer))
  (`TextBlock.SetText` (`/Game/MyContent/MapsManager/MapsFrancoisGuillaume/Levels/Lobby/UI_Lobby.txtNbrJoueur` (`self.UI_LobbyREF`)) (`KismetTextLibrary.Conv_StringToText` (`KismetStringLibrary.Concat_StrStr` "Players  " (`KismetStringLibrary.Conv_IntToString` nbrPlayer) " / " (`KismetStringLibrary.Conv_IntToString` nbrMaxPlayer)))))

(event `AffichePseudo`
  (`self.InitStruct`)
  (bind _asps_lobby (cast `/Game/MyContent/MapsManager/MapsFrancoisGuillaume/Levels/Lobby/PS_Lobby` (`Controller.PlayerState` (`GameplayStatics.GetPlayerController` 0))))
  (bind _ascharacter_car_cube (cast `/Game/MyContent/MapsManager/MapsFrancoisGuillaume/Levels/Lobby/Character_CarCube` (`self.K2_GetPawn` (`GameplayStatics.GetPlayerController` 0))))
  (bind (_structureplayer_id _structureplayer_username) (break `/Game/MyContent/MapsManager/MapsFrancoisGuillaume/Levels/LobbySystem/Structure/Structure_Player` (`/Game/MyContent/MapsManager/MapsFrancoisGuillaume/Levels/Lobby/PS_Lobby.structurePlayer` _asps_lobby)))
  (`self.S_AffichePseudo` _structureplayer_username _ascharacter_car_cube))

(event `S_AffichePseudo`
  (params (username :type String) (car :type "/Game/MyContent/MapsManager/MapsFrancoisGuillaume/Levels/Lobby/Character_CarCube Object Reference"))
  (`self.M_AffichePseudo` username car))

(event `M_AffichePseudo`
  (params (username :type String) (car :type "/Game/MyContent/MapsManager/MapsFrancoisGuillaume/Levels/Lobby/Character_CarCube Object Reference"))
  (bind _asui_username (cast `/Game/MyContent/MapsManager/MapsFrancoisGuillaume/Levels/Menu/UI_Username` (`WidgetComponent.GetWidget` (`/Game/MyContent/MapsManager/MapsFrancoisGuillaume/Levels/Lobby/Character_CarCube.WidgetUsername` car))))
  (`TextBlock.SetText` (`/Game/MyContent/MapsManager/MapsFrancoisGuillaume/Levels/Menu/UI_Username.txtNoName` _asui_username) (`KismetTextLibrary.Conv_StringToText` username)))

(event `AfficheColor`
  (bind _asps_lobby (cast `/Game/MyContent/MapsManager/MapsFrancoisGuillaume/Levels/Lobby/PS_Lobby` (`Controller.PlayerState` (`GameplayStatics.GetPlayerController` 0))))
  (bind _ascharacter_car_cube (cast `/Game/MyContent/MapsManager/MapsFrancoisGuillaume/Levels/Lobby/Character_CarCube` (`self.K2_GetPawn` (`GameplayStatics.GetPlayerController` 0))))
  (bind (_structureplayer_id _structureplayer_username _structureplayer_material) (break `/Game/MyContent/MapsManager/MapsFrancoisGuillaume/Levels/LobbySystem/Structure/Structure_Player` (`/Game/MyContent/MapsManager/MapsFrancoisGuillaume/Levels/Lobby/PS_Lobby.structurePlayer` _asps_lobby)))
  (`self.S_AfficheColor` _ascharacter_car_cube _structureplayer_material))

(event `S_AfficheColor`
  (params (Car :type "/Game/MyContent/MapsManager/MapsFrancoisGuillaume/Levels/Lobby/Character_CarCube Object Reference") (Material :type "Material Object Reference"))
  (`self.M_AfficheColor` Car Material))

(event `M_AfficheColor`
  (params (Car :type "/Game/MyContent/MapsManager/MapsFrancoisGuillaume/Levels/Lobby/Character_CarCube Object Reference") (Color :type "Material Object Reference"))
  (`PrimitiveComponent.SetMaterial` (`/Game/MyContent/MapsManager/MapsFrancoisGuillaume/Levels/Lobby/Character_CarCube.Cube` Car) 0 Color))

(event `S_CompteRebours`
  (params (second :type Integer))
  (`self.M_CompteRebours` second))

(event `M_CompteRebours`
  (params (second :type Integer))
  (`TextBlock.SetText` (`/Game/MyContent/MapsManager/MapsFrancoisGuillaume/Levels/Lobby/UI_Lobby.TxtCountdown` (`self.UI_LobbyREF`)) (`KismetTextLibrary.Conv_StringToText` (`KismetStringLibrary.Conv_IntToString` second))))

(event `M_DebutPartie`
  (bind _ascharacter_car_cube (cast `/Game/MyContent/MapsManager/MapsFrancoisGuillaume/Levels/Lobby/Character_CarCube` (`self.K2_GetPawn` (`GameplayStatics.GetPlayerController` 0))))
  (set `/Game/MyContent/MapsManager/MapsFrancoisGuillaume/Levels/Lobby/Character_CarCube.isMoveEnable` true _ascharacter_car_cube)
  (`TextBlock.SetText` (`/Game/MyContent/MapsManager/MapsFrancoisGuillaume/Levels/Lobby/UI_Lobby.TxtCountdown` (`self.UI_LobbyREF`)) ""))

(event `S_DebutPartie`
  (`self.M_DebutPartie`))

(fn `InitStruct`
  (bind _asgi_player (cast `/Game/MyContent/MapsManager/MapsFrancoisGuillaume/Levels/Menu/GI_Player` (`GameplayStatics.GetGameInstance`)))
  (bind _asps_lobby (cast `/Game/MyContent/MapsManager/MapsFrancoisGuillaume/Levels/Lobby/PS_Lobby` (`Controller.PlayerState` (`GameplayStatics.GetPlayerController` 0))))
  (bind _structureplayer_id (break `/Game/MyContent/MapsManager/MapsFrancoisGuillaume/Levels/LobbySystem/Structure/Structure_Player` (`/Game/MyContent/MapsManager/MapsFrancoisGuillaume/Levels/Lobby/PS_Lobby.structurePlayer` _asps_lobby)))
  (bind (_structure_player_id _structure_player_username _structure_player_material) (break `/Game/MyContent/MapsManager/MapsFrancoisGuillaume/Levels/LobbySystem/Structure/Structure_Player` (`/Game/MyContent/MapsManager/MapsFrancoisGuillaume/Levels/Menu/GI_Player.structure_Player` _asgi_player)))
  (set `/Game/MyContent/MapsManager/MapsFrancoisGuillaume/Levels/Lobby/PS_Lobby.structurePlayer` (make `/Game/MyContent/MapsManager/MapsFrancoisGuillaume/Levels/LobbySystem/Structure/Structure_Player` _structureplayer_id _structure_player_username _structure_player_material) _asps_lobby))

(fn `OnRep_usernamePlayer`
  (bind _ascharacter_car_cube (cast `/Game/MyContent/MapsManager/MapsFrancoisGuillaume/Levels/Lobby/Character_CarCube` (`self.K2_GetPawn`)))
  (bind _asui_username (cast `/Game/MyContent/MapsManager/MapsFrancoisGuillaume/Levels/Menu/UI_Username` (`WidgetComponent.GetWidget` (`/Game/MyContent/MapsManager/MapsFrancoisGuillaume/Levels/Lobby/Character_CarCube.WidgetUsername` _ascharacter_car_cube))))
  (`TextBlock.SetText` (`/Game/MyContent/MapsManager/MapsFrancoisGuillaume/Levels/Menu/UI_Username.txtNoName` _asui_username) (`KismetTextLibrary.Conv_StringToText` (`self.usernamePlayer`))))

(fn `UserConstructionScript`)