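; Car pawn Blueprint, named as a duplicate, whose only live logic plays an FMOD gravity-change sound.
; Space bar and gamepad left shoulder both play that event attached to its FMODAudio component; no gravity change happens in this graph.
; Disconnected nodes hold a speed HUD widget and an FMOD engine sound that follows the car, with horizontal speed driving its RPM parameter.
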(event `self.ReceiveBeginPlay`)

(event `self.ReceiveTick`
  (params (DeltaSeconds :type "Float (single-precision)")))

(event `Key|SpaceBar`
  (params (Key :type "Key Structure"))
  (:`Pressed`
    (`FMODBlueprintStatics.PlayEventAttached` "/Game/FMOD/Events/VEHICULE/Action/Action_Changement_Gravité.Action_Changement_Gravité" (`self.FMODAudio`) "None" (0.0 0.0 0.0) "KeepRelativeOffset")))

(event `Key|Gamepad_LeftShoulder`
  (params (Key :type "Key Structure"))
  (:`Pressed`
    (`FMODBlueprintStatics.PlayEventAttached` "/Game/FMOD/Events/VEHICULE/Action/Action_Changement_Gravité.Action_Changement_Gravité" (`self.FMODAudio`) "None" (0.0 0.0 0.0) "KeepRelativeOffset")))

(fn `UserConstructionScript`)