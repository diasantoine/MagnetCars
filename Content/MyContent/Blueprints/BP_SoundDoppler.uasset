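; BP_SoundDoppler is a world-placed actor that plays the Piste_DopplerWhoosh audio event at its own location and varies it with the player car's speed.
; BeginPlay finds the MyPawnCar, creates the event instance and starts it.
; Each Tick feeds the horizontal length of the car's collision velocity into the event's "RPM" parameter, or prints "FAIL" when the car is invalid.
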(event `self.ReceiveBeginPlay`
  (bind _returnvalue (`GameplayStatics.GetActorOfClass` "/Script/MagnetCars.MyPawnCar"))
  (set `self.PawnCar` _returnvalue)
  (bind _returnvalue_2 (`FMODBlueprintStatics.PlayEventAtLocation` "/Game/FMOD/Events/ARENA/Piste/1General/Piste_DopplerWhoosh.Piste_DopplerWhoosh" (`KismetMathLibrary.Conv_VectorToTransform` (`self.K2_GetActorLocation`))))
  (`FMODBlueprintStatics.EventInstancePlay` _returnvalue_2))

(event `self.ReceiveTick`
  (params (DeltaSeconds :type "Float (single-precision)"))
  (bind _pawncar (`self.PawnCar`))
  (bind (_returnvalue_x _returnvalue_y _returnvalue_z) (`KismetMathLibrary.BreakVector` (`SceneComponent.GetComponentVelocity` (`MyPawnCar.CarCollision` _pawncar))))
  (if (`KismetSystemLibrary.IsValid` _pawncar)
    (`FMODBlueprintStatics.EventInstanceSetParameter` (stale `self.ReceiveBeginPlay` _returnvalue_2) "RPM" (`KismetMathLibrary.VSizeXY` (`KismetMathLibrary.MakeVector` _returnvalue_x _returnvalue_y _returnvalue_z)))
    (else
      (`KismetSystemLibrary.PrintString` "FAIL"))))

(fn `UserConstructionScript`)