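; Player car pawn that layers FMOD audio, high-speed camera shake and a map-choice menu onto gravity-switching, boostable driving.
; BeginPlay starts engine and music events for the local player, opens the menu and fills the raycast point arrays.
; Tick feeds velocity to engine RPM and, when unboosted at high speed, shakes the camera and sets music SlowMotion from grounded state.
; Boost and gravity events trigger sounds; drift audio is disconnected.
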(event `Key|M`
  (params (Key :type "Key Structure"))
  (:`Pressed`
    (`FMODBlueprintStatics.EventInstanceSetParameter` (stale `self.ReceiveBeginPlay` _returnvalue_4) "VolPourcent")))

(event `Key|L`
  (params (Key :type "Key Structure"))
  (:`Pressed`
    (`FMODBlueprintStatics.EventInstanceSetParameter` (stale `self.ReceiveBeginPlay` _returnvalue_4) "VolPourcent" 100.0)))

(event `self.CarBoost`
  ;[1 1 1] Son moteur
  ;;[1 1 1] BOOST
  (`FMODBlueprintStatics.EventInstanceSetParameter` (stale `self.ReceiveBeginPlay` _returnvalue_3) "PriseBoost" 1.0))

(event `self.ReceiveBeginPlay`
  (bind _arrayhoziontalraycastposition (`self.ArrayHoziontalRaycastPosition`))
  (bind _arrayverticalraycastposition (`self.ArrayVerticalRaycastPosition`))
  (bind _returnvalue (`KismetMathLibrary.Conv_VectorToTransform` (`self.K2_GetActorLocation`)))
  (`|ExecutionSequence`
    (:`then_0`
      (set `self.TemporaryScene` (`self.Scene`))
      (bind _asplayer_controller (cast `PlayerController` (`self.GetController`)))
      (if (`Controller.IsLocalPlayerController` _asplayer_controller)
        (bind _returnvalue_2 (`|CreateWidget` "/Game/MyContent/Blueprints/WBP_ChoiceMap.WBP_ChoiceMap_C" _asplayer_controller (`self.CarCollision`)))
        (bind _output_get (set `self.WPB_MenuSpawnCircuit` _returnvalue_2))
        (`UserWidget.AddToViewport` _output_get 0)
        ;[1 1 1] Son moteur
        (bind _returnvalue_3 (`FMODBlueprintStatics.PlayEventAtLocation` "/Game/FMOD/Events/VEHICULE/Moteur/Moteur_Vitesse.Moteur_Vitesse" _returnvalue))
        (`FMODBlueprintStatics.EventInstancePlay` _returnvalue_3)
        (bind _returnvalue_4 (`FMODBlueprintStatics.PlayEventAtLocation` "/Game/FMOD/Events/ARENA/Environnement/Env_Music.Env_Music" _returnvalue))
        (`FMODBlueprintStatics.EventInstancePlay` _returnvalue_4)))
    (:`then_1`
      (`KismetArrayLibrary.Array_Add` _arrayverticalraycastposition (`self.Scene1`))
      (`KismetArrayLibrary.Array_Add` _arrayverticalraycastposition (`self.Scene2`))
      (`KismetArrayLibrary.Array_Add` _arrayhoziontalraycastposition (`self.Scene3`))
      (`KismetArrayLibrary.Array_Add` _arrayhoziontalraycastposition (`self.Scene4`)))))

(event `self.ReceiveTick`
  (params (DeltaSeconds :type "Float (single-precision)"))
  (bind _returnvalue (`GameplayStatics.GetPlayerCameraManager` 0))
  (bind _carstruct_isgrounded (break `Car` (`self.CarStruct`)))
  (bind (_carstruct_isgrounded_2 _carstruct_isleancreaterotation _carstruct_isrotationupactivewhengrounded _carstruct_isleancreateslow _carstruct_isonreversegravity _carstruct_instantreversegravity _carstruct_dragwholebodywhenlean _carstruct_isboosted) (break `Car` (`self.CarStruct`)))
  (bind (_returnvalue_x _returnvalue_y) (`KismetMathLibrary.BreakVector` (`SceneComponent.GetComponentVelocity` (`self.CarCollision`))))
  (bind (_returnvalue_x_2 _returnvalue_y_2 _returnvalue_z) (`KismetMathLibrary.BreakVector` (`SceneComponent.GetComponentVelocity` (`self.CarCollision`))))
  (`|ExecutionSequence`
    (:`then_0`
      ;[1 1 1] Son moteur
      (`FMODBlueprintStatics.EventInstanceSetTransform` (stale `self.ReceiveBeginPlay` _returnvalue_3) (`KismetMathLibrary.Conv_VectorToTransform` (`self.K2_GetActorLocation`)))
      (`FMODBlueprintStatics.EventInstanceSetParameter` (stale `self.ReceiveBeginPlay` _returnvalue_3) "RPM" (`KismetMathLibrary.VSize` (`KismetMathLibrary.MakeVector` _returnvalue_x_2 _returnvalue_y_2 _returnvalue_z)))
      ;[1 1 1] Reset parameter boost
      (if (not _carstruct_isboosted)
        (`FMODBlueprintStatics.EventInstanceSetParameter` (stale `self.ReceiveBeginPlay` _returnvalue_3) "PriseBoost")
        (if (> (`KismetMathLibrary.VSize` (`KismetMathLibrary.MakeVector` _returnvalue_x _returnvalue_y)) 5000.0)
          (bind _returnvalue_2 (`PlayerCameraManager.StartCameraShake` :`self` _returnvalue :`ShakeClass` "/Game/MyContent/Blueprints/BP_CameraShake.BP_CameraShake_C" :`Scale` 0.2))
          (set `self.BPCameraShake` _returnvalue_2)
          (if _carstruct_isgrounded
            (`FMODBlueprintStatics.EventInstanceSetParameter` (stale `self.ReceiveBeginPlay` _returnvalue_4) "SlowMotion")
            (else
              (`FMODBlueprintStatics.EventInstanceSetParameter` (stale `self.ReceiveBeginPlay` _returnvalue_4) "SlowMotion" 1.0)))
          (elif true
            (`PlayerCameraManager.StopAllCameraShakes` _returnvalue true)))))))

(event `self.CarReverseGravity`
  ;[1 1 1] Son switch
  (`FMODBlueprintStatics.PlayEventAttached` "/Game/FMOD/Events/VEHICULE/Action/Action_Changement_Gravité.Action_Changement_Gravité" (`self.FMODAudio`) "None" (0.0 0.0 0.0) "KeepRelativeOffset"))

(event `Key|N`
  (params (Key :type "Key Structure"))
  (:`Pressed`
    (if (`self.Keyboard`)
      (set `self.Keyboard` false)
      (else
        (set `self.Keyboard` true)))))

(fn `UserConstructionScript`)