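; BP_FrancoisCar is a car Blueprint that shows its current horizontal speed in a UI text field.
; Every Tick, it takes the XY velocity length of CarCollision, rounds it to a whole number and writes it to VelocityCar on the WPBMenuSpawnCircuit widget.
; An unconnected chain would create the WBP_ChoiceMap widget, link it to BP_LoadCircuit and set that reference, but it never runs.
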(event `self.ReceiveBeginPlay`)

(event `self.ReceiveTick`
  (params (DeltaSeconds :type "Float (single-precision)"))
  (bind (_returnvalue_x _returnvalue_y) (`KismetMathLibrary.BreakVector` (`SceneComponent.GetComponentVelocity` (`self.CarCollision`))))
  (`TextBlock.SetText` (`/Game/MyContent/Blueprints/WBP_ChoiceMap.VelocityCar` (`self.WPB_MenuSpawnCircuit`)) (`KismetTextLibrary.Conv_DoubleToText` (`KismetMathLibrary.VSize` (`KismetMathLibrary.MakeVector` _returnvalue_x _returnvalue_y)) "HalfToEven" false true 1 324 0 0)))

(fn `UserConstructionScript`)