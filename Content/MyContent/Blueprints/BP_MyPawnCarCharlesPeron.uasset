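; Networked player car pawn with drift, gravity flip and respawn inputs, gated by IsEnable and passed to movement functions defined outside this graph.
; Each tick the locally controlled car packs its transform state and relays it through server/multicast events, teleporting other copies to match.
; FMOD engine audio follows the car, using speed as RPM plus a boost parameter.
; When not boosted, high horizontal speed triggers camera shake.
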(event `S_CarBoost`
  (`self.M_CarBoost`))

(event `M_CarBoost`)

(event `S_MoteurSon`
  (params (location :type "Transform Structure"))
  (`self.M_MoteurSon` location))

(event `M_MoteurSon`
  (params (location :type "Transform Structure")))

(event `S_ColisionSound`
  (params (location :type "Transform Structure") (value :type "Float (double-precision)"))
  (`self.M_ColisionSound` location value))

(event `M_ColisionSound`
  (params (location :type "Transform Structure") (value :type "Float (double-precision)")))

(event `self.CarBoost`
  ;[1 1 1] Son moteur
  ;;[1 1 1] BOOST
  (`FMODBlueprintStatics.EventInstanceSetParameter` (stale `self.ReceiveBeginPlay` _returnvalue) "PriseBoost" 1.0))

(event `self.ReceiveBeginPlay`
  (bind _arrayverticalraycastposition (`self.ArrayVerticalRaycastPosition`))
  (bind _arrayhoziontalraycastposition (`self.ArrayHoziontalRaycastPosition`))
  (`|ExecutionSequence`
    (:`then_0`
      (set `self.TemporaryScene` (`self.Scene`))
      ;[1 1 1] Son moteur
      (bind _returnvalue (`FMODBlueprintStatics.PlayEventAtLocation` "/Game/FMOD/Events/VEHICULE/Moteur/Moteur_Vitesse.Moteur_Vitesse" (`KismetMathLibrary.Conv_VectorToTransform` (`self.K2_GetActorLocation`))))
      (`FMODBlueprintStatics.EventInstancePlay` _returnvalue))
    (:`then_1`
      (`KismetArrayLibrary.Array_Add` _arrayverticalraycastposition (`self.Scene1`))
      (`KismetArrayLibrary.Array_Add` _arrayverticalraycastposition (`self.Scene2`))
      (`KismetArrayLibrary.Array_Add` _arrayhoziontalraycastposition (`self.Scene3`))
      (`KismetArrayLibrary.Array_Add` _arrayhoziontalraycastposition (`self.Scene4`)))))

(event `self.ReceiveTick`
  (params (DeltaSeconds :type "Float (single-precision)"))
  (bind _returnvalue (`GameplayStatics.GetPlayerCameraManager` 0))
  (bind (_carstruct_isgrounded _carstruct_isleancreaterotation _carstruct_isrotationupactivewhengrounded _carstruct_isleancreateslow _carstruct_isonreversegravity _carstruct_instantreversegravity _carstruct_dragwholebodywhenlean _carstruct_isboosted) (break `Car` (`self.CarStruct`)))
  (bind (_returnvalue_x _returnvalue_y) (`KismetMathLibrary.BreakVector` (`SceneComponent.GetComponentVelocity` (`self.CarCollision`))))
  (`self.MovementManager`)
  ;[1 1 1] Son moteur
  (`self.MoteurSoundManager`)
  (`FMODBlueprintStatics.EventInstanceSetTransform` (stale `self.ReceiveBeginPlay` _returnvalue) (`self.LocationSound`))
  (`FMODBlueprintStatics.EventInstanceSetParameter` (stale `self.ReceiveBeginPlay` _returnvalue) "RPM" (`self.ColisionSound`))
  ;[1 1 1] Reset parameter boost
  (if (not _carstruct_isboosted)
    (`FMODBlueprintStatics.EventInstanceSetParameter` (stale `self.ReceiveBeginPlay` _returnvalue) "PriseBoost")
    (if (> (`KismetMathLibrary.VSize` (`KismetMathLibrary.MakeVector` _returnvalue_x _returnvalue_y)) 5000.0)
      (bind _returnvalue_2 (`PlayerCameraManager.StartCameraShake` :`self` _returnvalue :`ShakeClass` "/Game/MyContent/Blueprints/BP_CameraShake.BP_CameraShake_C" :`Scale` 0.2))
      (set `self.BPCameraShake` _returnvalue_2)
      (elif true
        (`PlayerCameraManager.StopAllCameraShakes` _returnvalue true)))))

(event `CustomEvent_0`
  (params (NewParam :type "/Game/MyContent/MapsManager/MapsFrancoisGuillaume/Levels/Lobby/StructStatCar Structure"))
  (set `self.structCarStat` NewParam))

(event `S_ModifServerSound`
  (params (NewParam :type "Transform Structure") (NewParam2 :type "Float (double-precision)"))
  (set `self.LocationSound` NewParam)
  (set `self.ColisionSound` NewParam2))

(event `self.CarReverseGravity`
  ;[1 1 1] Son switch
  (if (`self.IsLocallyControlled`)
    (`/Engine/EditorBlueprintResources/ActorMacros.Switch Has Authority`
      (:`Authority`
        (`self.M_CarReverseGravity`))
      (:`Remote`
        (`self.S_CarReverseGravity`)))))

(event `S_CarReverseGravity`
  (`self.M_CarReverseGravity`))

(event `M_CarReverseGravity`
  (`FMODBlueprintStatics.PlayEventAttached` "/Game/FMOD/Events/VEHICULE/Action/Action_Changement_Gravité.Action_Changement_Gravité" (`self.FMODAudio`) "None" (0.0 0.0 0.0) "KeepRelativeOffset"))

(event `Key|N`
  (params (Key :type "Key Structure")))

(event `M_LocAndRot`
  (bind (_structcarstat_position _structcarstat_rotation _structcarstat_velocity _structcarstat_rotationcollision _structcarstat_rotationmesh) (break `/Game/MyContent/MapsManager/MapsFrancoisGuillaume/Levels/Lobby/StructStatCar` (`self.structCarStat`)))
  (if (not (`self.IsLocallyControlled`))
    (`self.K2_SetActorLocationAndRotation` _structcarstat_position _structcarstat_rotation false true)
    (`SceneComponent.K2_SetRelativeRotation` (`self.CarCollision`) _structcarstat_rotationcollision false false)
    (`SceneComponent.K2_SetRelativeRotation` (`self.SkeletalMesh`) _structcarstat_rotationmesh false false)))

(event `S_LocAndRot`
  (`self.M_LocAndRot`))

(event `InputAxis|Forward`
  (params (AxisValue :type "Float (single-precision)"))
  (if (`self.isEnable`)
    (`self.ForwardMovement` AxisValue)
    (else
      (`self.ForwardMovement` 0.0))))

(event `InputAxis|Right`
  (params (AxisValue :type "Float (single-precision)"))
  (if (`self.isEnable`)
    (`self.RightMovement` AxisValue)
    (else
      (`self.RightMovement` 0.0))))

(event `InputAxis|LeftLean`
  (params (AxisValue :type "Float (single-precision)"))
  (if (`self.isEnable`)
    (`self.CarDrift` AxisValue)
    (else
      (`self.CarDrift` 0.0))))

(event `InputAxis|RightLean`
  (params (AxisValue :type "Float (single-precision)"))
  (if (`self.isEnable`)
    (`self.CarDrift` AxisValue)
    (else
      (`self.CarDrift` 0.0))))

(event `InputAction|ChangeGravity`
  (params (Key :type "Key Structure"))
  (:`Pressed`
    (if (`self.isEnable`)
      (`self.CarGravity`))))

(event `InputAction|ResetScene`
  (params (Key :type "Key Structure"))
  (:`Pressed`
    (`KismetSystemLibrary.PrintString` "Hello")))

(event `InputAction|Respawn`
  (params (Key :type "Key Structure"))
  (:`Pressed`
    (if (`self.isEnable`)
      (`self.CarRespawn`))))

(event `InputAxis|LookUp`
  (params (AxisValue :type "Float (single-precision)"))
  (if (`self.isEnable`)
    (`self.UpMovement` AxisValue)))

(fn `MoteurSoundManager`
  (bind (_returnvalue_x _returnvalue_y _returnvalue_z) (`KismetMathLibrary.BreakVector` (`SceneComponent.GetComponentVelocity` (`self.CarCollision`))))
  (if (`self.IsLocallyControlled`)
    (bind _output_get (set `self.LocationSound` (`KismetMathLibrary.Conv_VectorToTransform` (`self.K2_GetActorLocation`))))
    (bind _output_get_2 (set `self.ColisionSound` (`KismetMathLibrary.VSize` (`KismetMathLibrary.MakeVector` _returnvalue_x _returnvalue_y _returnvalue_z))))
    (`self.S_ModifServerSound` _output_get _output_get_2)
    (`/Engine/EditorBlueprintResources/ActorMacros.Switch Has Authority`)))

(fn `MovementManager`
  (if (`self.IsLocallyControlled`)
    (bind _output_get (set `self.structCarStat` (make `/Game/MyContent/MapsManager/MapsFrancoisGuillaume/Levels/Lobby/StructStatCar` (`self.K2_GetActorLocation`) (`self.GetControlRotation`) (`self.GetVelocity`) (`SceneComponent.RelativeRotation` (`self.CarCollision`)) (`SceneComponent.RelativeRotation` (`self.Scene`)))))
    (`self.CustomEvent_0` _output_get)
    (`/Engine/EditorBlueprintResources/ActorMacros.Switch Has Authority`
      (:`Authority`
        (`self.M_LocAndRot`))
      (:`Remote`
        (`self.S_LocAndRot`)))))

(fn `UserConstructionScript`)